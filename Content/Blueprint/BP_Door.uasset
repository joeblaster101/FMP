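; BP_Door is a door that slides open while an actor that passes a key check is inside its trigger box.
; BeginPlay caches the BP_FirstPersonCharacter, which IsActorWithKeyCheck takes with the overlapping actor on both begin and end overlap.
; A passing check plays or reverses a Timeline that lerps the mesh's relative X location.
; A game instance cast is left unconnected.
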(event OnComponentBeginOverlap(Box)
  (params (OverlappedComponent :type Primitive%20Component%20Object%20Reference) (OtherActor :type Actor%20Object%20Reference) (OtherComp :type Primitive%20Component%20Object%20Reference) (OtherBodyIndex :type Integer) (bFromSweep :type Boolean) (SweepResult :type Hit%20Result%20Structure%20%28by%20ref%29))
  (bind _outputflow (Class|Door|IsActorwithKeyCheck OtherActor (Variables|Default|Getcharacture)))
  (if _outputflow
    (bind _newtrack_0 (Timeline|Timeline Play)
      (:Update
        (Transformation|SetRelativeLocation (Variables|Default|GetStaticMesh) (Math|Vector|MakeVector (Math|Float|Lerp 0.0 2e+02 _newtrack_0) 0.0 0.0) false false)))))

(event OnComponentEndOverlap(Box)
  (params (OverlappedComponent :type Primitive%20Component%20Object%20Reference) (OtherActor :type Actor%20Object%20Reference) (OtherComp :type Primitive%20Component%20Object%20Reference) (OtherBodyIndex :type Integer))
  (bind _outputflow (Class|Door|IsActorwithKeyCheck OtherActor (Variables|Default|Getcharacture)))
  (if _outputflow
    (bind _newtrack_0 (Timeline|Timeline Reverse)
      (:Update
        (Transformation|SetRelativeLocation (Variables|Default|GetStaticMesh) (Math|Vector|MakeVector (Math|Float|Lerp 0.0 2e+02 _newtrack_0) 0.0 0.0) false false)))))

(event EventBeginPlay
  (bind _returnvalue (Actor|GetActorOfClass "/Game/FirstPerson/Blueprints/BP_FirstPersonCharacter.BP_FirstPersonCharacter_C"))
  (Variables|Default|Setcharacture _returnvalue))

(fn ConstructionScript)