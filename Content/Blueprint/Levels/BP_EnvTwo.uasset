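; BP_EnvTwo is an environment Blueprint that hands a set of spawn markers to the game instance when play begins.
; On BeginPlay it casts to BP_GameInstance, caches the reference and appends its four Billboard components to a Spawns array.
; It then passes that array to the game instance's Begin function, which receives all further control, as this Blueprint has no other logic.
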(event EventBeginPlay
  (bind _asbp_game_instance (Utilities|Casting|CastToBP_GameInstance (Game|GetGameInstance)))
  (Variables|Default|SetGame%20Instance _asbp_game_instance)
  (Utilities|Array|AppendArray (Variables|Default|Getspawns) (Utilities|Array|MakeArray (Variables|Default|GetBillboard) (Variables|Default|GetBillboard1) (Variables|Default|GetBillboard2) (Variables|Default|GetBillboard3)))
  (Default|Begin (Variables|Default|GetGame%20Instance) (Variables|Default|Getspawns)))

(fn ConstructionScript)