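; Base enemy Blueprint that chases the first-person player and fires a gun.
; On BeginPlay it caches the player and loops AI MoveTo toward them, reissuing on success or failure.
; While HasShot is set, Tick fires after a short delay, using either a Billboard-origin hitscan trace or an AI bullet spawn.
; Projectiles are aimed by the player camera's rotation, and hit handling is an empty stub.
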(event Custom|GunTick
  ;[0.1016 0 1] gun 1
  (if (Variables|Default|GetbHasShot)
    (Utilities|FlowControl|Delay 0.02)
    (if (Variables|Default|GetIsHitscan)
      (bind _outhit (|hitscanGun))
      (|hit _outhit)
      (else
        (|shootprjectile)))))

(event Custom|trigger%20move
  ;[0.5937 1 0] ai moving
  (AI|AIMoveTo self (.Location (Math|Transform|BreakTransform (Variables|Default|GetPlayerLocation))) (Variables|Default|Getplayer) 5.0 false
    (:OnSuccess
      _)
    (:OnFail
      _))
  (CallFunction|TriggerMove))

(event EventTick
  (params (DeltaSeconds :type Float%20%28single-precision%29))
  (CallFunction|GunTick)
  (Variables|Default|SetPlayerLocation (|PlayerLocationNodes)))

(event EventBeginPlay
  (Utilities|FlowControl|Sequence
    (:then_0
      (bind _returnvalue (Actor|GetActorOfClass "/Game/FirstPerson/Blueprints/BP_FirstPersonCharacter.BP_FirstPersonCharacter_C"))
      (Variables|Default|Setplayer _returnvalue))
    (:then_1
      (CallFunction|TriggerMove))))

(fn ConstructionScript)