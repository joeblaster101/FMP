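; Parkour movement component that gives a Character wall running, vertical wall runs, ledge grabs, mantling and jump-offs.
; Once initialized, a looping 60 Hz timer drives wall checks, mantling and mode-based camera tilt through gates that jump, landing and movement events open or close.
; Traces find walls and ledges, then launches, gravity changes and interpolation move the character.
; A parkour mode enum tracks state, with timed gate reopening as cooldowns.
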(event Custom|Initialize
  (params (Character :type Character%20Object%20Reference))
  (bind _output_get (Variables|Default|SetCharacter Character))
  (Variables|Default|SetCharacterMovement (Variables|/Script/Engine.Character|GetCharacterMovement _output_get))
  (Variables|Default|SetDefaultGravity (Variables|/Script/Engine.CharacterMovementComponent|GetGravityScale (Variables|/Script/Engine.Character|GetCharacterMovement _output_get)))
  (Utilities|Time|SetTimerbyEvent (delegate Custom|WallRunUpdateEvent) 0.0167 true))

(event Custom|WallRunUpdateEvent
  (Utilities|FlowControl|Sequence
    (:then_0
      (|WallRunUpdates))
    (:then_1
      (|VerticalWallRun))
    (:then_2
      (|Mantle))
    (:then_3
      (CallFunction|CameraTick))))

(event Custom|Land%20Event
  (CallFunction|WallRunEnd 0.0)
  (CallFunction|VerticalWallRunEnd 0.0)
  (CallFunction|CloseGates)
  (CallFunction|PlayCameraShake "/Game/CameraShacks/BP_JumpLand.BP_JumpLand_C"))

(event Custom|Jump%20Event
  (if (Utilities|Enum|Equal(Enum) (Variables|Default|Getcurrent%20Parkour%20Movementmode) "NewEnumerator0")
    (if (not (AI|Components|NavMovement|IsFalling (Variables|Default|GetCharacterMovement)))
      (CallFunction|OpenGate)
      (CallFunction|PlayCameraShake "/Game/CameraShacks/BP_JumpLand.BP_JumpLand_C"))
    (else
      (CallFunction|JumpEvents))))

(event Custom|MoveMentChange
  (params (PreveouseMovement :type EMovementMode%20Enum :default "MOVE_None") (NewMovement :type EMovementMode%20Enum :default "MOVE_None"))
  (Utilities|IsValid (Variables|Default|GetCharacterMovement)
    (:Is%20Valid
      (Variables|Default|SetPreveouse%20Movement PreveouseMovement)
      (Variables|Default|Setcurrent%20MovementMode NewMovement)
      (|OpenAllGates))))

(event Custom|ParkourMovementChanged
  (params (PrevParkourMovementMode :type E_ParkoreMovement%20Enum :default "NewEnumerator0") (NewParkourMovementmode :type E_ParkoreMovement%20Enum :default "NewEnumerator0"))
  (Variables|Default|SetPrev%20Parkour%20Movement%20Mode PrevParkourMovementMode)
  (Variables|Default|Setcurrent%20Parkour%20Movementmode NewParkourMovementmode)
  (CallFunction|Reset))

(event Custom|PlayCameraShake
  (params (shake :type Legacy%20Camera%20Shake%20Class%20Reference))
  (if (Variables|Default|GetCameraShake)
    (Camera|PlayWorldCameraShake shake (Transformation|GetActorLocation (Variables|Default|GetCharacter)) 0.0 1e+02)))

(fn WallRunUpdate
  (if (Utilities|CanWallRun)
    (bind _onwall (CallFunction|WallRunMovement (Transformation|GetActorLocation (Variables|Default|GetCharacter)) (.Right (Utilities|WallRunEndVectors)) -1.0))
    (if _onwall ; Right WallRun
      (CallFunction|SetParkourMovementMode "NewEnumerator2")
      (CallFunction|WallRunGravity :!label _label)
      (elif (Utilities|Enum|Equal(Enum) (Variables|Default|Getcurrent%20Parkour%20Movementmode) "NewEnumerator2") ; No longer wall-running right.
        (CallFunction|WallRunEnd 0.5)
        (else
          (bind _onwall_2 (CallFunction|WallRunMovement (Transformation|GetActorLocation (Variables|Default|GetCharacter)) (.Left (Utilities|WallRunEndVectors)) 1.0))
          (if _onwall_2
            (CallFunction|SetParkourMovementMode "NewEnumerator1")
            (goto _label)
            (else
              (CallFunction|WallRunEnd 0.5))))))
    (else
      (CallFunction|WallRunEnd 1.0))))

(fn WallRunEnd
  (params (ResetTime :type Float%20%28double-precision%29))
  (if (Utilities|WallRunning?)
    (bind _change (CallFunction|SetParkourMovementMode "NewEnumerator0"))
    (if _change
      (CallFunction|CloseWallRunGate)
      (Utilities|Time|SetTimerbyFunctionName 0 "OpenWallRunGate" ResetTime))))

(fn WallRunMovement
  (params (Start :type Vector) (End :type Vector) (WallRunDirection :type Float%20%28double-precision%29))
  (bind _outhit (Collision|LineTraceByChannel Start End "TraceTypeQuery1" false 0 "None"))
  (if (.bblockinghit _outhit) ; Hit something?
    (Variables|WallRun|SetWallRunNormal (.OutVec (Utilities|ValidWallRunVector? (.normal _outhit))))
    (if (and (AI|Components|NavMovement|IsFalling (Variables|Default|GetCharacterMovement)) (.ReturnValue (Utilities|ValidWallRunVector? (.normal _outhit)))) ; Valid wall and falling?
      (Character|LaunchCharacter (Variables|Default|GetCharacter) (* (Math|Vector|CrossProduct (Variables|WallRun|GetWallRunNormal) "0, 0,1.000000") (* (Variables|WallRun|GetWallRunSpeed) WallRunDirection)) true (not (Variables|WallRun|GetWallRunGravity?))) ; Add forward force.
      (return true)
      (else
        (return false)))
    (else
      (return false))))

(fn WallRunGravity
  (Variables|/Script/Engine.CharacterMovementComponent|SetGravityScale (Variables|Default|GetCharacterMovement) (Math|Interpolation|FInterpTo (Variables|/Script/Engine.CharacterMovementComponent|GetGravityScale (Variables|Default|GetCharacterMovement)) (Variables|WallRun|GetWallRunTargetGravity) (Utilities|Time|GetWorldDeltaSeconds) (Variables|WallRun|GetWallRunStartSpeed))))

(fn CameraTilt
  (params (Target%20X%20%28Roll%29 :type Float%20%28double-precision%29))
  (bind _character (Variables|Default|GetCharacter))
  (bind _returnvalue (Pawn|GetController _character))
  (bind _returnvalue_2 (Pawn|GetControlRotation _returnvalue :!class /Script/Engine.Controller))
  (bind (_roll _pitch _yaw) (Math|Rotator|BreakRotator _returnvalue_2))
  (Pawn|SetControlRotation (Pawn|GetController (Variables|Default|GetCharacter)) (Math|Interpolation|RInterpTo _returnvalue_2 (Math|Rotator|MakeRotator Target%20X%20%28Roll%29 _pitch _yaw) (Utilities|Time|GetWorldDeltaSeconds) 1e+01))
  (return))

(fn CameraTick
  (switch Utilities|FlowControl|Switch|SwitchonE_ParkoreMovement (Variables|Default|Getcurrent%20Parkour%20Movementmode)
    (:NewEnumerator0
      (CallFunction|CameraTilt 0.0 :!label _label))
    (:NewEnumerator1
      (CallFunction|CameraTilt 15.0))
    (:NewEnumerator2
      (CallFunction|CameraTilt -15.0 :!label _label_2))
    (:NewEnumerator3
      (goto _label))
    (:NewEnumerator4
      (goto _label))
    (:NewEnumerator5
      (goto _label))
    (:NewEnumerator6
      (goto _label_2))
    (:NewEnumerator7
      (goto _label))))

(fn CameraReset
  (CallFunction|CameraTilt 0.0))

(fn WallRunJump
  (bind _wallrunjumpoffforce (Variables|WallRun|GetWallRunJumpOffForce))
  (bind _wallrunnormal (Variables|WallRun|GetWallRunNormal))
  (if (Utilities|WallRunning?)
    (CallFunction|WallRunEnd 0.35) ; Reset gravity and WallRunning bools
    (Utilities|IsValid (Variables|Default|GetCharacter)
      (:Is%20Valid
        (Character|LaunchCharacter (Variables|Default|GetCharacter) (Math|Vector|MakeVector (* _wallrunjumpoffforce (.x _wallrunnormal)) (* _wallrunjumpoffforce (.y _wallrunnormal)) (Variables|WallRun|GetWallRunJumpHeight)) false true) ; Launch character towards the camera's fwd direction.
      ))))

(fn Reset
  (if (Utilities|Enum|Equal(Enum) (Variables|Default|GetPrev%20Parkour%20Movement%20Mode) "NewEnumerator0")
    (Variables|/Script/Engine.CharacterMovementComponent|SetGravityScale (Variables|Default|GetCharacterMovement) (Variables|Default|GetDefaultGravity))
    (Pawn|Components|CharacterMovement|SetMovementMode (Variables|Default|GetCharacterMovement) (Utilities|Select :Index "NewEnumerator0" :NewEnumerator0 "MOVE_Falling" :NewEnumerator1 "MOVE_Falling" :NewEnumerator2 "MOVE_Falling" :NewEnumerator3 "MOVE_Falling" :NewEnumerator4 "MOVE_Falling" :NewEnumerator5 "MOVE_Walking" :NewEnumerator6 "MOVE_Walking" :NewEnumerator7 "MOVE_Walking") 0)))

(fn SetParkourMovementMode
  (params (NewMode :type E_ParkoreMovement%20Enum :default "NewEnumerator0"))
  (if (Utilities|Enum|Equal(Enum) NewMode (Variables|Default|Getcurrent%20Parkour%20Movementmode))
    (return false)
    (else
      (CallFunction|ParkourMovementChanged (Variables|Default|Getcurrent%20Parkour%20Movementmode) NewMode)
      (return true))))

(fn VerticlWallRunUpdate
  (bind (_eyes _feet) (Utilities|MantleVactors))
  (if (Utilities|WallRunning?)
    (bind (_outhit _returnvalue) (Collision|CapsuleTraceByChannel _eyes _feet 2e+01 1e+01 "TraceTypeQuery1" false 0 "None"))
    (if _returnvalue
      (Variables|Default|SetMantleTraceDistance (.Distance (Collision|BreakHitResult _outhit)))
      (if (not (Class|CharacterMovementComponent|IsWalkable (Variables|Default|GetCharacterMovement) _outhit))
        (CallFunction|VerticalWallRunMovemnet :!label _label)
        (Variables|Default|SetMantalPosition (+ (.ImpactPoint (Collision|BreakHitResult _outhit)) (Math|Vector|MakeVector 0.0 0.0 (Variables|/Script/Engine.CapsuleComponent|GetCapsuleHalfHeight (Variables|/Script/Engine.Character|GetCapsuleComponent (Variables|Default|GetCharacter))))))
        (|LedgeGrab)
        (if (Utilities|QuickMntle)
          (CallFunction|OpenMantleGate)
          (else
            (Utilities|Time|SetTimerbyFunctionName 0 "OpenMantleCheckGate" 0.25))))
      (else
        (goto _label)))
    (else
      (CallFunction|VerticalWallRunEnd 0.35))))

(fn VerticalWallRunEnd
  (params (reset%20time :type Float%20%28double-precision%29))
  (bind _current_parkour_movementmode (Variables|Default|Getcurrent%20Parkour%20Movementmode))
  (if (Math|Boolean|ORBoolean (Utilities|Enum|Equal(Enum) _current_parkour_movementmode "NewEnumerator4") (Utilities|Enum|Equal(Enum) _current_parkour_movementmode "NewEnumerator3") (Utilities|Enum|Equal(Enum) _current_parkour_movementmode "NewEnumerator5"))
    (bind _change (CallFunction|SetParkourMovementMode "NewEnumerator0"))
    (if _change
      (CallFunction|CloseVerticalWallRunGate)
      (CallFunction|CloseMantleGate)
      (Utilities|Time|SetTimerbyFunctionName 0 "OpenVerticalWallRunGate" reset%20time)
      (CallFunction|OpenVerticalWallRunGate))))

(fn VerticalWallRunMovemnet
  (bind _feet (Utilities|MantleVactors))
  (bind (_outhit _returnvalue) (Collision|LineTraceByChannel _feet (+ (* (Transformation|GetActorForwardVector (Variables|Default|GetCharacter)) (Variables|Default|Get50)) _feet) "TraceTypeQuery1" false 0 "None"))
  (if (and (> (Utilities|ForwardInput) 0.0) _returnvalue)
    (Variables|Default|SetVerticalWallRunNormal (.ImpactNormal (Collision|BreakHitResult _outhit)))
    (CallFunction|SetParkourMovementMode "NewEnumerator3")
    (Character|LaunchCharacter (Variables|Default|GetCharacter) (Math|Vector|MakeVector (.x (- (Variables|Default|GetVerticalWallRunNormal) -6e+02)) (.y (- (Variables|Default|GetVerticalWallRunNormal) -6e+02)) (Variables|Default|GetVerticalWallRunSpeed)) true true)
    (else
      (CallFunction|VerticalWallRunEnd 0.35))))

(fn MantleMovement
  (bind _character (Variables|Default|GetCharacter))
  (bind _character_2 (Variables|Default|GetCharacter))
  (bind _mantalposition (Variables|Default|GetMantalPosition))
  (bind _returnvalue (Pawn|GetController _character_2))
  (bind _returnvalue_2 (Transformation|GetActorLocation _character))
  (Pawn|SetControlRotation _returnvalue (Math|Interpolation|RInterpTo (Pawn|GetControlRotation _returnvalue :!class /Script/Engine.Controller) (Math|Rotator|FindLookatRotation (Math|Vector|MakeVector (.x _returnvalue_2) (.y _returnvalue_2) 0.0) (Math|Vector|MakeVector (.x _mantalposition) (.y _mantalposition) 0.0)) (Utilities|Time|GetWorldDeltaSeconds) 7.0))
  (Transformation|SetActorLocation (Variables|Default|GetCharacter) (Math|Interpolation|VInterpTo (Transformation|GetActorLocation (Variables|Default|GetCharacter)) (Variables|Default|GetMantalPosition) (Utilities|Time|GetWorldDeltaSeconds) (select (Utilities|QuickMntle) (Variables|Default|GetQuickMantalSpeed) (Variables|Default|GetStanderdMantalSpeed))) false false)
  (if (< (Math|Vector|Distance(Vector) (Transformation|GetActorLocation (Variables|Default|GetCharacter)) (Variables|Default|GetMantalPosition)) 8.0)
    (CallFunction|VerticalWallRunEnd 5.0)))

(fn OpenGate
  (CallFunction|OpenWallRunGate)
  (CallFunction|OpenVerticalWallRunGate))

(fn CloseGates
  (CallFunction|CloseWallRunGate)
  (CallFunction|CloseVerticalWallRunGate))

(fn LedgeGrabJump
  (bind _current_parkour_movementmode (Variables|Default|Getcurrent%20Parkour%20Movementmode))
  (bind _ledgegrabjumpoffforce (Variables|Default|GetLedgeGrabJumpOffForce))
  (bind _verticalwallrunnormal (Variables|Default|GetVerticalWallRunNormal))
  (if (Math|Boolean|ORBoolean (Utilities|Enum|Equal(Enum) _current_parkour_movementmode "NewEnumerator4") (Utilities|Enum|Equal(Enum) _current_parkour_movementmode "NewEnumerator3") (Utilities|Enum|Equal(Enum) _current_parkour_movementmode "NewEnumerator5"))
    (CallFunction|VerticalWallRunEnd 0.35)
    (Character|LaunchCharacter (Variables|Default|GetCharacter) (Math|Vector|MakeVector (* (.x _verticalwallrunnormal) _ledgegrabjumpoffforce) (* _ledgegrabjumpoffforce (.y _verticalwallrunnormal)) (Variables|Default|GetLedgeGrabJumpHight)) false false)))

(fn JumpEvents
  (CallFunction|WallRunJump)
  (CallFunction|LedgeGrabJump))

(event Custom|OpenMantleCheckGate
  (Utilities|FlowControl|Gate true) ; enters at Open
)

(event Custom|CloseMantleCheckGet
  (Utilities|FlowControl|Gate true) ; enters at Close
)

(event Custom|OpenMantleGate
  (Utilities|FlowControl|Gate true) ; enters at Open
)

(event Custom|CloseMantleGate
  (Utilities|FlowControl|Gate true) ; enters at Close
)

(event Custom|MantleCheck
  (if (Utilities|CanMantle)
    (CallFunction|MantleStart)))

(event Custom|MantleStart
  (bind _change (CallFunction|SetParkourMovementMode "NewEnumerator0"))
  (if _change
    (CallFunction|PlayCameraShake (select (Utilities|CanMantle) "/Game/CameraShacks/BP_QuickMantle.BP_QuickMantle_C" "/Game/CameraShacks/BP_Mantle.BP_Mantle_C"))
    (CallFunction|CloseMantleCheckGet)
    (CallFunction|OpenMantleGate)))

(event Custom|OpenWallRunGate
  (Utilities|FlowControl|Gate true) ; enters at Open
)

(event Custom|CloseWallRunGate
  (Utilities|FlowControl|Gate true) ; enters at Close
)

(event Custom|OpenVerticalWallRunGate
  (Utilities|FlowControl|Gate true) ; enters at Open
)

(event Custom|closeVerticalWallRunGate
  (CallFunction|CloseMantleGate)
  (Utilities|FlowControl|Gate true) ; enters at Close
)