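; BP_GunSpawner is an actor that spawns a weapon at its Billboard when a round ends.
; It caches BP_GameInstance on BeginPlay, then polls EndOfRound every Tick, with a DoOnce limiting spawns to one until that check turns false.
; WeaponSpawn receives the GunLevel result and the Billboard's world location and rotation.
; The endOfRound and gunLevel graphs contain only unused reads of the game instance's End and GunLevel.
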(event EventBeginPlay
  (bind _asbp_game_instance (Utilities|Casting|CastToBP_GameInstance (Game|GetGameInstance)))
  (Variables|Default|SetGameInstance _asbp_game_instance))

(event Collision|EventActorBeginOverlap
  (params (OtherActor :type Actor%20Object%20Reference)))

(event EventTick
  (params (DeltaSeconds :type Float%20%28single-precision%29))
  (bind _billboard (Variables|Default|GetBillboard))
  (bind _returnvalue (Transformation|GetWorldTransform _billboard))
  (if (Utilities|EndOfRound)
    (Utilities|FlowControl|DoOnce false :!label _label
      (:Completed
        (Class|GunSpawner|WeaponSpawn (Utilities|GunLevel) (.location _returnvalue) (.rotation _returnvalue))))
    (else
      (goto _label Reset))))

(fn ConstructionScript)