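; BP_PlayerTarget is an actor that serves as a marker for where the player was seen.
; On BeginPlay it waits a tick and caches the first-person player character.
; When SomeoneHasSeen fires, it stores the seen flag, moves to the character's CurrentLocation, prints a debug string, and clears the flag after a short delay.
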(event Custom|SomeoneHasSeen
  (params (Seeing :type Boolean))
  (Variables|Default|SetHasSeen Seeing)
  (Transformation|SetActorLocation (Variables|/Game/FirstPerson/Blueprints/BP_FirstPersonCharacter.BP_FirstPersonCharacter_C|GetCurrentLocation (Variables|Default|GetFirst%20Person%20Character)) false false)
  (Development|PrintString "Hello")
  (Utilities|FlowControl|Delay 0.2)
  (Variables|Default|SetHasSeen false))

(event EventBeginPlay
  (Utilities|FlowControl|DelayUntilNextTick)
  (bind _asbp_first_person_character (Utilities|Casting|CastToBP_FirstPersonCharacter (Game|GetPlayerCharacter 0)))
  (Variables|Default|SetFirst%20Person%20Character _asbp_first_person_character))

(fn ConstructionScript)