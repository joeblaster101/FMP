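; BP_LevlStart is a trigger actor that starts a round on the game instance when the first-person character enters its boxes.
; BeginPlay caches the game instance and character, and each of three box overlaps checks for that character.
; All three feed one shared DoOnce that calls ROUNDSTART.
; Tick re-arms that gate once whenever Target's HasPast becomes true, using a second DoOnce for edge detection.
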(event OnComponentBeginOverlap(Box)
  (params (OverlappedComponent :type Primitive%20Component%20Object%20Reference) (OtherActor :type Actor%20Object%20Reference) (OtherComp :type Primitive%20Component%20Object%20Reference) (OtherBodyIndex :type Integer) (bFromSweep :type Boolean) (SweepResult :type Hit%20Result%20Structure%20%28by%20ref%29))
  (bind _outputflow (Class|LevlStart|IsActorCheck OtherActor (Variables|Default|GetFirst%20Person%20Character)))
  (if _outputflow
    (Utilities|FlowControl|DoOnce false
      (:Completed
        (Default|ROUNDSTART (Variables|Default|GetGame%20Instance))))))

(event OnComponentBeginOverlap(Box1)
  (params (OverlappedComponent :type Primitive%20Component%20Object%20Reference) (OtherActor :type Actor%20Object%20Reference) (OtherComp :type Primitive%20Component%20Object%20Reference) (OtherBodyIndex :type Integer) (bFromSweep :type Boolean) (SweepResult :type Hit%20Result%20Structure%20%28by%20ref%29))
  (bind _outputflow (Class|LevlStart|IsActorCheck OtherActor (Variables|Default|GetFirst%20Person%20Character)))
  (if _outputflow
    (Utilities|FlowControl|DoOnce false
      (:Completed
        (Default|ROUNDSTART (Variables|Default|GetGame%20Instance))))))

(event OnComponentBeginOverlap(Box2)
  (params (OverlappedComponent :type Primitive%20Component%20Object%20Reference) (OtherActor :type Actor%20Object%20Reference) (OtherComp :type Primitive%20Component%20Object%20Reference) (OtherBodyIndex :type Integer) (bFromSweep :type Boolean) (SweepResult :type Hit%20Result%20Structure%20%28by%20ref%29))
  (bind _outputflow (Class|LevlStart|IsActorCheck OtherActor (Variables|Default|GetFirst%20Person%20Character)))
  (if _outputflow
    (Utilities|FlowControl|DoOnce false
      (:Completed
        (Default|ROUNDSTART (Variables|Default|GetGame%20Instance))))))

(event EventBeginPlay
  ;[0.7109 1 0] begin
  (bind _asbp_game_instance (Utilities|Casting|CastToBP_GameInstance (Game|GetGameInstance)))
  (Variables|Default|SetGame%20Instance _asbp_game_instance)
  (bind _returnvalue (Actor|GetActorOfClass "/Game/FirstPerson/Blueprints/BP_FirstPersonCharacter.BP_FirstPersonCharacter_C"))
  (Variables|Default|SetFirst%20Person%20Character _returnvalue))

(event EventTick
  (params (DeltaSeconds :type Float%20%28single-precision%29))
  (Utilities|FlowControl|Sequence
    (:then_0
      (if (Variables|/Game/Blueprint/BP_Target.BP_Target_C|GetHasPast (Variables|Default|GetTarget))
        (Utilities|FlowControl|DoOnce false :!label _label
          (:Completed
            (Utilities|FlowControl|DoOnce false) ; enters at Reset
          ))
        (else
          (goto _label Reset))))))

(fn ConstructionScript)